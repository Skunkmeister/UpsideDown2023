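; Base music looper actor that switches between a normal track and an upside-down track when the world flips sides.
; Two audio components hold the tracks and replay from the start on finishing, with the upside-down one paused at BeginPlay.
; FlipSides runs a timeline on both volumes, swaps which component is paused, then ramps volume with a second timeline.
; Pausing rather than stopping lets each track resume where it left off.
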(event `self.ReceiveBeginPlay`
  (bind _volume (`self.volume`))
  (`parent.ReceiveBeginPlay`)
  (`AudioComponent.SetSound` (`self.Real Audio`) (`self.Normal Sound`))
  (`AudioComponent.SetVolumeMultiplier` (`self.Real Audio`) _volume)
  (`AudioComponent.SetSound` (`self.UpDnAudio`) (`self.UpDn Sound`))
  (`AudioComponent.SetVolumeMultiplier` (`self.UpDnAudio`) _volume)
  (`AudioComponent.SetPaused` (`self.UpDnAudio`) true))

(event `self.Real Audio.OnAudioFinished`
  (`AudioComponent.Play` (`self.Real Audio`) 0.0))

(event `self.FlipSides`
  (params (`isNowUpsideDown?` :type Boolean))
  (bind (_direction _newtrack_0) (`Timeline|Timeline` :!via `PlayFromStart`)
    (:`Update`
      (bind _returnvalue (* _newtrack_0 (`self.volume`)))
      (`AudioComponent.SetVolumeMultiplier` (`self.Real Audio`) _returnvalue)
      (`AudioComponent.SetVolumeMultiplier` (`self.UpDnAudio`) _returnvalue))
    (:`Finished`
      (`AudioComponent.SetPaused` (`self.UpDnAudio`) (not `isNowUpsideDown?`))
      (`AudioComponent.SetPaused` (`self.Real Audio`) `isNowUpsideDown?`)
      (bind (_direction_2 _newtrack_0_2) (`Timeline|volume ramp up` :!via `PlayFromStart`)
        (:`Update`
          (bind _returnvalue_2 (* _newtrack_0_2 (`self.volume`)))
          (`AudioComponent.SetVolumeMultiplier` (`self.Real Audio`) _returnvalue_2)
          (`AudioComponent.SetVolumeMultiplier` (`self.UpDnAudio`) _returnvalue_2))))))

(event `self.UpDnAudio.OnAudioFinished`
  (`AudioComponent.Play` (`self.UpDnAudio`) 0.0))

(fn `UserConstructionScript`
  (`parent.UserConstructionScript`))