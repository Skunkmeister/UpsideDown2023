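; Base pickup actor that grants the player an item (flashlight, watch, key or intel) and ties its availability to the normal or upside-down dimension.
; With SingleDimensionVisibility set, it is visible and enabled only in the dimension matching its UD flag, re-evaluated by FlipSides.
; Any sphere overlap while enabled sets the matching flag on the cached first-person character, without checking the overlapping actor, then destroys the pickup.
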(event `self.ReceiveBeginPlay`
  (bind _returnvalue (`KismetMathLibrary.BooleanNAND` (`self.UD?`) (`self.Single Dimension Visibility`)))
  (`parent.ReceiveBeginPlay`)
  (bind _asbp_first_person_character (cast `/Game/Blueprints/Player/BP_FirstPersonCharacter` (`GameplayStatics.GetPlayerCharacter` 0)))
  (set `self.As BP First Person Character` _asbp_first_person_character)
  (set `self.enabled` _returnvalue)
  (`self.SetActorHiddenInGame` (not _returnvalue)))

(event `self.FlipSides`
  (params (`isNowUpsideDown?` :type Boolean))
  (bind _returnvalue (not (`self.Single Dimension Visibility`)))
  (bind _returnvalue_2 (or (and `isNowUpsideDown?` (or _returnvalue (`self.UD?`))) (and _returnvalue (`self.UD?`)) (and (not (`self.UD?`)) (not `isNowUpsideDown?`))))
  (`self.SetActorHiddenInGame` (not _returnvalue_2))
  (set `self.enabled` _returnvalue_2))

(event `self.Sphere.OnComponentBeginOverlap`
  (params (OverlappedComponent :type "PrimitiveComponent Object Reference") (OtherActor :type "Actor Object Reference") (OtherComp :type "PrimitiveComponent Object Reference") (OtherBodyIndex :type Integer) (bFromSweep :type Boolean) (SweepResult :type "HitResult Structure (by ref)"))
  (bind _as_bp_first_person_character (`self.As BP First Person Character`))
  (if (`self.enabled`)
    (switch `/Game/Blueprints/Player/InventoryEnum` (`self.Enables Item`)
      (:`NewEnumerator0`
        (set `/Game/Blueprints/Player/BP_FirstPersonCharacter.Has Flashlight` true _as_bp_first_person_character))
      (:`NewEnumerator1`
        (set `/Game/Blueprints/Player/BP_FirstPersonCharacter.haswatch` true _as_bp_first_person_character))
      (:`NewEnumerator2`
        (set `/Game/Blueprints/Player/BP_FirstPersonCharacter.hasbluekey` true _as_bp_first_person_character))
      (:`NewEnumerator3`
        (set `/Game/Blueprints/Player/BP_FirstPersonCharacter.hasredkey` true _as_bp_first_person_character))
      (:`NewEnumerator4`
        (set `/Game/Blueprints/Player/BP_FirstPersonCharacter.hasintel` true _as_bp_first_person_character)))
    (`self.K2_DestroyActor`)))

(fn `UserConstructionScript`
  (`parent.UserConstructionScript`))