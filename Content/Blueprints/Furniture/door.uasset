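; An interactable door that may require a blue key, a red key or both from the first-person character.
; A per-tick polling loop from BeginPlay checks distance, keys and the character's RequestDoorOpen flag.
; A nearby prompt widget shows "Locked!" tinted by the missing key colours.
; Valid requests alternate open and close via FlipFlop, with sound, rotation timelines and a handle morph, and polling resumes when the swing finishes.
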(event `self.ReceiveBeginPlay`
  (bind _as_open_dialog_widget (`self.As Open Dialog Widget`))
  (bind _returnvalue (or (`/Game/Blueprints/Player/BP_FirstPersonCharacter.hasredkey` (`self.As BP First Person Character`)) (not (`self.Requires Red Key`))))
  (bind _returnvalue_2 (or (`/Game/Blueprints/Player/BP_FirstPersonCharacter.hasbluekey` (`self.As BP First Person Character`)) (not (`self.Requires Blue Key`))))
  (bind _returnvalue_3 (and _returnvalue_2 _returnvalue))
  (bind _returnvalue_4 (< (`KismetMathLibrary.Vector_Distance` (`self.K2_GetActorLocation` (`Controller.K2_GetPawn` (`GameplayStatics.GetPlayerController` 0))) (`self.K2_GetActorLocation`)) 200.0))
  (`|ExecutionSequence`
    (:`then_0`
      (bind _asbp_first_person_character (cast `/Game/Blueprints/Player/BP_FirstPersonCharacter` (`GameplayStatics.GetPlayerCharacter` 0))
        (:`then`
          (set `self.As BP First Person Character` _asbp_first_person_character))
        (:`CastFailed`
          (`KismetSystemLibrary.PrintString` "CAST FAIL"))))
    (:`then_1`
      (bind _asopen_dialog_widget (cast `/Game/UI/openDialogWidget` (`WidgetComponent.GetUserWidgetObject` (`self.open dialog`))))
      (set `self.As Open Dialog Widget` _asopen_dialog_widget)
      ;[1 1 1] Loops back from timers
      (if (and _returnvalue_4 (`/Game/Blueprints/Player/BP_FirstPersonCharacter.Request Door Open` (`self.As BP First Person Character`)) _returnvalue_3) :!label _label
        (set `/Game/Blueprints/Player/BP_FirstPersonCharacter.Request Door Open` false (`self.As BP First Person Character`))
        (`|ExecutionSequence`
          (:`then_0`
            (`/Engine/EditorBlueprintResources/StandardMacros.FlipFlop`
              (:`A`
                (`GameplayStatics.PlaySound2D` "/Game/Sounds/open_door.open_door" 1.0 1.0 0.0 null null)
                (bind (_direction _door_angle) (`Timeline|Open Door` :!via `PlayFromStart`)
                  (:`Update`
                    (`SceneComponent.K2_SetRelativeRotation` (`self.Block-Door__2_`) (`KismetMathLibrary.MakeRotator` 0.0 0.0 _door_angle) false false))
                  (:`Finished`
                    (goto _label))))
              (:`B`
                (`GameplayStatics.PlaySound2D` "/Game/Sounds/close_door.close_door" 1.0 1.0 0.0 null null)
                (bind (_direction_2 _closing) (`Timeline|Close Door` :!via `PlayFromStart`)
                  (:`Update`
                    (`SceneComponent.K2_SetRelativeRotation` (`self.Block-Door__2_`) (`KismetMathLibrary.MakeRotator` 0.0 0.0 _closing) false false))
                  (:`Finished`
                    (goto _label))))))
          (:`then_1`
            (bind (_direction_3 _newtrack_0) (`Timeline|Adjust Handle` :!via `PlayFromStart`)
              (:`Update`
                (`SkeletalMeshComponent.SetMorphTarget` (`self.Block-Door__2_`) "TurnHandle" _newtrack_0 true)))))
        (else
          (`KismetSystemLibrary.DelayUntilNextTick`)
          (`SceneComponent.SetVisibility` (`self.open dialog`) _returnvalue_4 false)
          (set `/Game/UI/openDialogWidget.statusText` (`KismetMathLibrary.SelectString` "" "Locked!" _returnvalue_3) _as_open_dialog_widget)
          (set `/Game/UI/openDialogWidget.statusTextColor` (make `SlateColor` (+ (`KismetMathLibrary.SelectColor` (struct) (struct :`G` 0.059021 :`B` 1.0 :`A` 1.0) _returnvalue_2) (`KismetMathLibrary.SelectColor` (struct) (struct :`R` 1.0 :`B` 0.081419 :`A` 1.0) _returnvalue))) _as_open_dialog_widget)
          (goto _label))))))

(fn `UserConstructionScript`)