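; Collapsed terrain furniture piece whose rock blocker appears only when it is flipped upside down.
; BlockRock starts hidden without collision at BeginPlay, and FlipSides toggles its visibility and query-and-physics collision to match the upside-down state.
; The construction script gives the rock a random world rotation on all three axes for visual variety.
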(event `self.ReceiveBeginPlay`
  (`parent.ReceiveBeginPlay`)
  (`SceneComponent.SetVisibility` (`self.Block-Rock`) false false)
  (`PrimitiveComponent.SetCollisionEnabled` (`self.Block-Rock`) "NoCollision" :!label _label))

(event `self.FlipSides`
  (params (`isNowUpsideDown?` :type Boolean))
  (`SceneComponent.SetVisibility` (`self.Block-Rock`) `isNowUpsideDown?` false)
  (if `isNowUpsideDown?`
    (`PrimitiveComponent.SetCollisionEnabled` (`self.Block-Rock`) "QueryAndPhysics")
    (else
      (goto _label))))

(fn `UserConstructionScript`
  (`parent.UserConstructionScript`)
  (`SceneComponent.K2_SetWorldRotation` (`self.Block-Rock`) (`KismetMathLibrary.MakeRotator` (`KismetMathLibrary.RandomFloatInRange` -180.0 180.0) (`KismetMathLibrary.RandomFloatInRange` -180.0 180.0) (`KismetMathLibrary.RandomFloatInRange` -180.0 180.0)) false false))