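; Beast NPC that appears only while the world is upside down and chases the player.
; On BeginPlay it binds to the iSpyGameState global flip event, which sets its upside-down flag and hides or shows the actor.
; While flipped, each Tick writes its location to a global material parameter collection as BeastPosition, then issues a navmesh move to a random point near the player.
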(event `self.ReceiveBeginPlay`
  ;[1 1 1] Receive Boolean on whether UD or Not
  (bind _asi_spy_game_state (cast `/Game/Blueprints/iSpyGameState` (`GameplayStatics.GetGameState`)))
  (add `/Game/Blueprints/iSpyGameState.flipUDGlobal` _asi_spy_game_state (delegate `SetUD`)))

(event `SetUD`
  (params (`isNowUpsideDown?` :type Boolean))
  ;[1 1 1] Receive Boolean on whether UD or Not
  (bind _output_get (set `self.upsideDown?` `isNowUpsideDown?`))
  (`self.SetActorHiddenInGame` (not _output_get)))

(event `self.ReceiveTick`
  (params (DeltaSeconds :type "Float (single-precision)"))
  (if (`self.upsideDown?`)
    (`self.Update Material Beast Position`)
    (`|ExecutionSequence`
      (:`then_0`
        (if true
          ;[1 1 1] Move to a random spot near the player
          (bind _randomlocation (`NavigationSystemV1.K2_GetRandomLocationInNavigableRadius` (`self.K2_GetActorLocation` (`Controller.K2_GetPawn` (`GameplayStatics.GetPlayerController` 0))) 20.0 null null))
          (`AIBlueprintHelperLibrary.SimpleMoveToLocation` (`self.GetController`) _randomlocation))))))

(fn `Update Material Beast Position`
  (`KismetMaterialLibrary.SetVectorParameterValue` "/Game/Materials/GlobalMaterialVars.GlobalMaterialVars" "BeastPosition" (make `LinearColor` (.x (`self.K2_GetActorLocation`)) (.y (`self.K2_GetActorLocation`)) (.z (`self.K2_GetActorLocation`)))))

(fn `UserConstructionScript`)