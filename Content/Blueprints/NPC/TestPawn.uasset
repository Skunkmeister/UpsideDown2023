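; TestPawn is an NPC test pawn with two waypoint components and a PawnSensing component, largely unimplemented.
; On BeginPlay it hides both waypoints; Tick, overlap and sensing events are empty.
; An unconnected node chain sketches a view-cone check, comparing the angle between a viewpoint direction and the direction to the player against a threshold.
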(event `self.ReceiveTick`
  (params (DeltaSeconds :type "Float (single-precision)")))

(event `self.ReceiveBeginPlay`
  (`SceneComponent.SetVisibility` (`self.waypoint1`) false false)
  (`SceneComponent.SetVisibility` (`self.waypoint2`) false false))

(event `self.PawnSensing.OnSeePawn`
  (params (Pawn :type "Pawn Object Reference")))

(event `self.PawnSensing.OnHearNoise`
  (params (Instigator :type "Pawn Object Reference") (Location :type "Vector Structure (by ref)") (Volume :type "Float (single-precision)")))

(fn `UserConstructionScript`)