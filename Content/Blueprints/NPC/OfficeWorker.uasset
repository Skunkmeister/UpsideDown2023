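; OfficeWorker is an NPC that patrols, chases the player once seen and damages them at close range.
; Tick switches walk and idle animations by velocity, moves through target offsets from its construction location on a delay, or follows the player after PawnSensing spots them.
; A game state flip event hides and freezes it while upside down, restoring it after a delay when flipped back.
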(event `Freeze and Hide`
  (params (`isNowUpsideDown?` :type Boolean))
  (if `isNowUpsideDown?`
    (`self.SetActorHiddenInGame` true)
    (set `self.frozen?` true)
    (else
      (`KismetSystemLibrary.Delay` 2.0)
      (`self.SetActorHiddenInGame` false)
      (set `self.frozen?` false))))

(event `self.ReceiveBeginPlay`
  (bind _asi_spy_game_state (cast `/Game/Blueprints/iSpyGameState` (`GameplayStatics.GetGameState`)))
  (add `/Game/Blueprints/iSpyGameState.flipUDGlobal` _asi_spy_game_state (delegate `Freeze and Hide`)))

(event `self.PawnSensing.OnSeePawn`
  (params (Pawn :type "Pawn Object Reference"))
  (if (not (`self.frozen?`))
    (bind _asbp_first_person_character (cast `/Game/Blueprints/Player/BP_FirstPersonCharacter` Pawn)
      (:`then`
        (set `self.As BP First Person Character` _asbp_first_person_character)
        (set `self.FOUNDYOU` true)
        (`KismetSystemLibrary.PrintString` "saw PLAYER"))
      (:`CastFailed`
        (`KismetSystemLibrary.PrintString` "saw not player")))))

(event `self.ReceiveTick`
  (params (DeltaSeconds :type "Float (single-precision)"))
  (bind _returnvalue (`self.GetController`))
  (bind _mesh (`self.Mesh`))
  (bind _targetlocations (`self.TargetLocations`))
  (if (not (`self.frozen?`))
    (`|ExecutionSequence`
      (:`then_0`
        ;[1 1 1] Update Animation in Accordance with Velocity
        (if (> (`KismetMathLibrary.VSize` (`CharacterMovementComponent.GetLastUpdateVelocity` (`self.CharacterMovement`))) 10.0)
          (`SkeletalMeshComponent.SetAnimation` _mesh "/Game/Blueprints/NPC/A_Walk.A_Walk")
          (else
            (`SkeletalMeshComponent.SetAnimation` _mesh "/Game/Blueprints/NPC/A_Idle.A_Idle"))))
      (:`then_1`
        (if (`self.FOUNDYOU`)
          (`AIBlueprintHelperLibrary.SimpleMoveToLocation` _returnvalue (`self.K2_GetActorLocation` (`Controller.K2_GetPawn` (`GameplayStatics.GetPlayerController` 0))))
          (else
            (`AIBlueprintHelperLibrary.SimpleMoveToLocation` _returnvalue (+ (`|GetArrayItem` _targetlocations (`self.Target Location Index`)) (`self.offsetLoc`)))
            (`KismetSystemLibrary.Delay` 5.0)
            (bind _result (`/Engine/EditorBlueprintResources/StandardMacros.IncrementInt` (`self.Target Location Index`))
              (:`  `
                (bind _output_get (set `self.Target Location Index` (mod _result (`KismetArrayLibrary.Array_Length` _targetlocations))))
                (`KismetSystemLibrary.PrintString` (`KismetStringLibrary.Concat_StrStr` "moving to" (`KismetStringLibrary.Conv_IntToString` _output_get))))))))
      (:`then_2`
        (`/Engine/EditorBlueprintResources/StandardMacros.CompareFloat` (`KismetMathLibrary.Vector_Distance` (`self.K2_GetActorLocation` (`Controller.K2_GetPawn` (`GameplayStatics.GetPlayerController` 0))) (`self.K2_GetActorLocation`)) 100.0
          (:`<`
            (`KismetSystemLibrary.Delay` 0.2)
            (`/Game/Blueprints/Player/BP_FirstPersonCharacter.TakeDamage` (`self.As BP First Person Character`) 20.0)))))))

(fn `UserConstructionScript`
  (set `self.offsetLoc` (`self.K2_GetActorLocation`)))